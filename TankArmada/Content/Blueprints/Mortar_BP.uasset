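; Mortar Blueprint actor with an aimable turret and barrel, a health pool and a health bar widget.
; On BeginPlay it passes the barrel and turret to the MortarAiming component, links itself to the HealthBar widget and binds to any-damage events.
; Damage is rounded and clamped to remaining health, and the mortar destroys itself at zero.
; GetPercentHealth returns current health as a fraction of starting health.
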(event `self.ReceiveBeginPlay`
  ;[1 1 1] Initialize
  (`TankAimingComponent.Initialize` (`self.Mortar Aiming`) (`self.MortarBarrel`) (`self.MortarTurret`))
  (`self.InitializeHealthBar`)
  (bind _output_get (set `self.CurrentHealth` (`self.StartingHealth`)))
  ;[1 1 1] Damage System
  (add `self.OnTakeAnyDamage` (delegate `OnTakeAnyDamage_Event_0`)))

(event `OnTakeAnyDamage_Event_0` :!signature `self.OnTakeAnyDamage`
  (params (DamagedActor :type "Actor Object Reference") (Damage :type "Float (double-precision)") (DamageType :type "DamageType Object Reference") (InstigatedBy :type "Controller Object Reference") (DamageCauser :type "Actor Object Reference"))
  ;[1 1 1] Damage System
  (bind _output_get (set `self.CurrentHealth` (- (stale `self.ReceiveBeginPlay` _output_get) (`KismetMathLibrary.Clamp` (`KismetMathLibrary.Round` Damage) 0 (stale `self.ReceiveBeginPlay` _output_get)))))
  (if (== _output_get 0)
    (`self.K2_DestroyActor`)))

(fn `GetPercentHealth`
  (returns (CurrentHealth :type "Float (double-precision)"))
  (return (/ (`KismetMathLibrary.Conv_IntToDouble` (`self.CurrentHealth`)) (`KismetMathLibrary.Conv_IntToDouble` (`self.StartingHealth`)))))

(fn `InitializeHealthBar`
  (bind _ashealth_bar (cast `/Game/UI/HealthBar` (`WidgetComponent.GetUserWidgetObject` (`self.Health Bar`))))
  (set `/Game/UI/HealthBar.Mortar` self _ashealth_bar)
  (return))

(fn `UserConstructionScript`)